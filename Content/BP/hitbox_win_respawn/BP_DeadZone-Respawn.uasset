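; BP_DeadZone-Respawn is a trigger zone that sends both balls back to their start points when either one falls into it.
; Two seconds after BeginPlay it finds and caches the BP_Ball and BP_Ball1 actors.
; When either ball begins overlapping its Box, both are teleported without sweep to StartPoint and StartPoint2 respectively.
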(event OnComponentBeginOverlap(Box)
  (params (OverlappedComponent :type Primitive%20Component%20Object%20Reference) (OtherActor :type Actor%20Object%20Reference) (OtherComp :type Primitive%20Component%20Object%20Reference) (OtherBodyIndex :type Integer) (bFromSweep :type Boolean) (SweepResult :type Hit%20Result%20Structure%20%28by%20ref%29))
  (if (or (== OtherActor (Variables|Default|GetBall1)) (== OtherActor (Variables|Default|GetBall2)))
    (Transformation|SetActorLocation (Variables|Default|GetBall1) (Transformation|GetActorLocation (Variables|Default|GetStartPoint)) false true)
    (Transformation|SetActorLocation (Variables|Default|GetBall2) (Transformation|GetActorLocation (Variables|Default|GetStartPoint_2)) false true)))

(event EventBeginPlay
  (Utilities|FlowControl|Delay 2.0)
  (bind _returnvalue (Actor|GetActorOfClass "/Game/BP/BP_Car/BP_CarEtLink/BP_Ball.BP_Ball_C"))
  (Variables|Default|SetBall1 _returnvalue)
  (bind _returnvalue_2 (Actor|GetActorOfClass "/Game/BP/BP_Car/BP_CarEtLink/BP_Ball1.BP_Ball1_C"))
  (Variables|Default|SetBall2 _returnvalue_2))

(fn ConstructionScript)