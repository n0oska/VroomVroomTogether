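; BP_Link acts as an elastic tether between the BP_Car and BP_Car2 actors.
; Shortly after BeginPlay it finds both cars and stores their current separation as the maximum distance.
; Each Tick, when they exceed that distance, it pulls their meshes together with opposing forces scaled by the offset between them, printing a debug string.
; Unconnected nodes would move the actor to the cars' midpoint.
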(event EventBeginPlay
  (Utilities|FlowControl|Delay 0.2)
  (bind _returnvalue (Actor|GetActorOfClass "/Game/BP/BP_Car/BP_Car.BP_Car_C"))
  (Variables|Default|SetBP_Car1 _returnvalue)
  (bind _returnvalue_2 (Actor|GetActorOfClass "/Game/BP/BP_Car/BP_Car2.BP_Car2_C"))
  (Variables|Default|SetBP_car2 _returnvalue_2)
  (Variables|Default|SetDistMax (Math|Vector|Distance(Vector) (Transformation|GetActorLocation (Variables|Default|GetBP_Car1)) (Transformation|GetActorLocation (Variables|Default|GetBP_car2)))))

(event EventTick
  (params (DeltaSeconds :type Float%20%28single-precision%29))
  (Math|Float|CompareFloat (Math|Vector|Distance(Vector) (Transformation|GetActorLocation (Variables|Default|GetBP_Car1)) (Transformation|GetActorLocation (Variables|Default|GetBP_car2))) (Variables|Default|GetDistMax)
    (:>
      (Physics|AddForce (Variables|/Script/ChaosVehicles.WheeledVehiclePawn|GetMesh (Variables|Default|GetBP_car2)) (* (- (Transformation|GetActorLocation (Variables|Default|GetBP_Car1)) (Transformation|GetActorLocation (Variables|Default|GetBP_car2))) 7e+02) "None" false)
      (Physics|AddForce (Variables|/Script/ChaosVehicles.WheeledVehiclePawn|GetMesh (Variables|Default|GetBP_Car1)) (* (- (Transformation|GetActorLocation (Variables|Default|GetBP_car2)) (Transformation|GetActorLocation (Variables|Default|GetBP_Car1))) 7e+02) "None" false)
      (Development|PrintString "Hello"))))

(fn ConstructionScript)

(fn GetDistanceVector)