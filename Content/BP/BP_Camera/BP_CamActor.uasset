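; BP_CamActor is a camera rig actor that frames two cars, BP_Car and BP_Car2, together.
; It finds both cars shortly after BeginPlay, then each Tick takes their midpoint from a line trace's endpoints.
; It moves to a raised, fixed offset from that midpoint, shifted by the signed vector between the cars, and rotates toward the midpoint.
; Debug drawing of the midpoint and camera line runs every frame.
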(event EventBeginPlay
  (Utilities|FlowControl|Delay 0.2)
  (bind _returnvalue (Actor|GetActorOfClass "/Game/BP/BP_Car/BP_Car.BP_Car_C"))
  (Variables|Default|SetCar1 _returnvalue)
  (bind _returnvalue_2 (Actor|GetActorOfClass "/Game/BP/BP_Car/BP_Car2.BP_Car2_C"))
  (Variables|Default|SetCar2 _returnvalue_2))

(event EventTick
  (params (DeltaSeconds :type Float%20%28single-precision%29))
  (Utilities|IsValid (Variables|Default|GetCar1)
    (:Is%20Valid
      (Utilities|IsValid (Variables|Default|GetCar2)
        (:Is%20Valid
          (bind _outhit (Collision|LineTraceByChannel (Transformation|GetActorLocation (Variables|Default|GetCar1)) (Transformation|GetActorLocation (Variables|Default|GetCar2)) "TraceTypeQuery1" false 0 "None"))
          (bind _output_get (Variables|Default|SetCenter (+ (/ (- (.tracestart _outhit) (.traceend _outhit)) 2.0) (.traceend _outhit))))
          (Rendering|Debug|DrawDebugSphere _output_get 5e+01 12 "(R=1.000000,G=1.000000,B=1.000000,A=1.000000)" 1e+01 1.0)
          (Collision|LineTraceByChannel (Variables|Default|GetCenter) (- (+ (Variables|Default|GetCenter) "0.000000,0.000000,500.000000") (Math|Vector|MakeVector (+ (.X (Math|Vector|BreakVector (- (.traceend _outhit) (.tracestart _outhit)))) 3e+03) (+ (.Y (Math|Vector|BreakVector (- (.traceend _outhit) (.tracestart _outhit)))) -6e+02) (.Z (Math|Vector|BreakVector (- (.traceend _outhit) (.tracestart _outhit)))))) "TraceTypeQuery1" false 0 "ForOneFrame")
          (Transformation|SetActorLocationAndRotation (- (+ (Variables|Default|GetCenter) "0.000000,0.000000,500.000000") (Math|Vector|MakeVector (+ (.X (Math|Vector|BreakVector (- (.traceend _outhit) (.tracestart _outhit)))) 3e+03) (+ (.Y (Math|Vector|BreakVector (- (.traceend _outhit) (.tracestart _outhit)))) -6e+02) (.Z (Math|Vector|BreakVector (- (.traceend _outhit) (.tracestart _outhit)))))) (Math|Rotator|FindLookatRotation (Transformation|GetActorLocation) (Variables|Default|GetCenter))))))))

(fn ConstructionScript)