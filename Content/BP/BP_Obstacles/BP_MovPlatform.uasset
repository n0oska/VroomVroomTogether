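; BP_MovPlatform is a moving platform obstacle that shuttles its Cube back and forth.
; From BeginPlay, the Moving timeline sets the Cube's relative location without sweeping.
; A five-second Delay chained to the timeline's Update, not Finished, then flips IsLooping to alternate between Reverse and PlayFromStart.
; An actor overlap handler applies a small X-axis force to the Cube itself, not the overlapping actor.
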(event Custom|OnActorBeginOverlap_Event
  (params (OverlappedActor :type Actor%20Object%20Reference) (OtherActor :type Actor%20Object%20Reference))
  (Class|PrimitiveComponent|AddForceatLocation (Variables|Default|GetCube) "10.000000,0.000000,0.000000" (Transformation|GetActorLocation) "None"))

(event EventBeginPlay
  (bind _moving (Timeline|Moving Play)
    (:Update
      (Transformation|SetRelativeLocation (Variables|Default|GetCube) _moving false false)
      (Utilities|FlowControl|Delay 5.0)
      (if (Variables|Default|GetIsLooping)
        (Variables|Default|SetIsLooping false)
        (Timeline|Moving Reverse)
        (else
          (Variables|Default|SetIsLooping true)
          (Timeline|Moving PlayFromStart))))))

(fn ConstructionScript)