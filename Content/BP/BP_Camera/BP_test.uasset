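; Test actor that acts as an elastic tether between BP_Car and BP_Car2.
; Shortly after BeginPlay it finds both cars and stores their separation as the maximum distance.
; When Tick finds them farther apart, it pulls each mesh toward the other with force scaled by their offset.
; It then moves itself to their midpoint, derived from a line trace's endpoints, with debug print and sphere.
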(event EventBeginPlay
  (Utilities|FlowControl|Delay 0.2)
  (bind _returnvalue (Actor|GetActorOfClass "/Game/BP/BP_Car/BP_Car.BP_Car_C"))
  (Variables|Default|SetBP_Car1 _returnvalue)
  (bind _returnvalue_2 (Actor|GetActorOfClass "/Game/BP/BP_Car/BP_Car2.BP_Car2_C"))
  (Variables|Default|SetBP_car2 _returnvalue_2)
  (Variables|Default|SetDistMax (Math|Vector|Distance(Vector) (Transformation|GetActorLocation (Variables|Default|GetBP_Car1)) (Transformation|GetActorLocation (Variables|Default|GetBP_car2)))))

(event EventTick
  (params (DeltaSeconds :type Float%20%28single-precision%29))
  (Math|Float|CompareFloat (Math|Vector|Distance(Vector) (Transformation|GetActorLocation (Variables|Default|GetBP_Car1)) (Transformation|GetActorLocation (Variables|Default|GetBP_car2))) (Variables|Default|GetDistMax)
    (:>
      (Physics|AddForce (Variables|/Script/ChaosVehicles.WheeledVehiclePawn|GetMesh (Variables|Default|GetBP_car2)) (* (- (Transformation|GetActorLocation (Variables|Default|GetBP_Car1)) (Transformation|GetActorLocation (Variables|Default|GetBP_car2))) 7e+02) "None" false)
      (Physics|AddForce (Variables|/Script/ChaosVehicles.WheeledVehiclePawn|GetMesh (Variables|Default|GetBP_Car1)) (* (- (Transformation|GetActorLocation (Variables|Default|GetBP_car2)) (Transformation|GetActorLocation (Variables|Default|GetBP_Car1))) 7e+02) "None" false)
      (Development|PrintString "Hello")
      (bind _outhit (Collision|LineTraceByChannel (Transformation|GetActorLocation (Variables|Default|GetBP_Car1)) (Transformation|GetActorLocation (Variables|Default|GetBP_car2)) "TraceTypeQuery1" false 0 "None"))
      (bind _output_get (Variables|Default|SetCenter (+ (/ (- (.tracestart _outhit) (.traceend _outhit)) 2.0) (.traceend _outhit))))
      (Rendering|Debug|DrawDebugSphere _output_get 5e+01 12 "(R=1.000000,G=1.000000,B=1.000000,A=1.000000)" 1e+01 1.0)
      (Transformation|SetActorLocation _output_get false false))))

(fn ConstructionScript)

(fn GetDistanceVector)