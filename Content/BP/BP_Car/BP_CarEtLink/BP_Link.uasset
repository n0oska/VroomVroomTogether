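; BP_Link is an actor that acts as an elastic tether between BP_Car and BP_Car2.
; Shortly after BeginPlay it finds both cars and stores their starting separation as the maximum distance.
; On Tick, beyond that distance, it pulls their meshes together with forces scaled by the offset, more strongly on BP_Car2.
; An unconnected trace chain would move the link to their midpoint.
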(event EventBeginPlay
  (Utilities|FlowControl|Delay 0.2)
  (bind _returnvalue (Actor|GetActorOfClass "/Game/BP/BP_Car/BP_CarEtLink/BP_Car.BP_Car_C"))
  (Variables|Default|SetBP_Car1 _returnvalue)
  (bind _returnvalue_2 (Actor|GetActorOfClass "/Game/BP/BP_Car/BP_CarEtLink/BP_Car2.BP_Car2_C"))
  (Variables|Default|SetBP_car2 _returnvalue_2)
  (Variables|Default|SetDistMax (Math|Vector|Distance(Vector) (Transformation|GetActorLocation (Variables|Default|GetBP_Car1)) (Transformation|GetActorLocation (Variables|Default|GetBP_car2)))))

(event EventTick
  (params (DeltaSeconds :type Float%20%28single-precision%29))
  (Utilities|IsValid (Variables|Default|GetBP_Car1)
    (:Is%20Valid
      (Utilities|IsValid (Variables|Default|GetBP_car2)
        (:Is%20Valid
          (Math|Float|CompareFloat (Math|Vector|Distance(Vector) (Transformation|GetActorLocation (Variables|Default|GetBP_Car1)) (Transformation|GetActorLocation (Variables|Default|GetBP_car2))) (Variables|Default|GetDistMax)
            (:>
              (Physics|AddForce (Variables|/Script/ChaosVehicles.WheeledVehiclePawn|GetMesh (Variables|Default|GetBP_car2)) (* (- (Transformation|GetActorLocation (Variables|Default|GetBP_Car1)) (Transformation|GetActorLocation (Variables|Default|GetBP_car2))) 5e+02) "None" false)
              (Physics|AddForce (Variables|/Script/ChaosVehicles.WheeledVehiclePawn|GetMesh (Variables|Default|GetBP_Car1)) (* (- (Transformation|GetActorLocation (Variables|Default|GetBP_car2)) (Transformation|GetActorLocation (Variables|Default|GetBP_Car1))) 1.5e+02) "None" false))))))))

(fn ConstructionScript)

(fn GetDistanceVector)