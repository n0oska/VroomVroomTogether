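; GM_Vehicle is the game mode for a two-player local vehicle game with a race timer.
; On BeginPlay it creates a second local player, spawns BP_Car and BP_Car2 at fixed positions, and has each player controller possess one car.
; Tick adds delta time to Racetime while IsWin is true; nothing in this graph sets that flag.
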(event EventBeginPlay
  (bind _returnvalue (Class|GameplayStatics|CreatePlayer 1))
  (bind _returnvalue_2 (Game|SpawnActorfromClass "/Game/BP/BP_Car/BP_CarEtLink/BP_Car.BP_Car_C" (Math|Transform|MakeTransform "0.000000,760.000000,0.000000" "0, 0, 0" "1.000000,1.000000,1.000000") "Undefined" "MultiplyWithRoot" 0 0))
  (Pawn|Possess (Game|GetPlayerController 0) _returnvalue_2)
  (bind _returnvalue_3 (Game|SpawnActorfromClass "/Game/BP/BP_Car/BP_CarEtLink/BP_Car2.BP_Car2_C" (Math|Transform|MakeTransform "0.000000,1320.000000,0.000000" "0, 0, 0" "1.000000,1.000000,1.000000") "Undefined" "MultiplyWithRoot" 0 0))
  (Pawn|Possess _returnvalue _returnvalue_3))

(event EventTick
  (params (DeltaSeconds :type Float%20%28single-precision%29))
  (if (Variables|Default|GetIsWin)
    (Variables|Default|SetRacetime (+ DeltaSeconds (Variables|Default|GetRacetime)))))

(fn ConstructionScript)