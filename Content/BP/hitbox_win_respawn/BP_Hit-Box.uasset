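; BP_Hit-Box is a win trigger that ends the game when a BP_Ball or BP_Ball1 overlaps its box.
; Either cast flags IsWin on GM_Vehicle, then creates WBP_Win with a coin total summed from both cast outputs and the time from the WBP_Timer found after BeginPlay.
; It then pauses the game and focuses input on the win screen.
; The ball references cached at BeginPlay go unused here.
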(event OnComponentBeginOverlap(Box)
  (params (OverlappedComponent :type Primitive%20Component%20Object%20Reference) (OtherActor :type Actor%20Object%20Reference) (OtherComp :type Primitive%20Component%20Object%20Reference) (OtherBodyIndex :type Integer) (bFromSweep :type Boolean) (SweepResult :type Hit%20Result%20Structure%20%28by%20ref%29))
  (Utilities|FlowControl|Sequence
    (:then_0
      (bind _asbp_ball (Utilities|Casting|CastToBP_Ball OtherActor)))
    (:then_1
      (bind _asbp_ball_1 (Utilities|Casting|CastToBP_Ball1 OtherActor))))
  (bind _asgm_vehicle (Utilities|Casting|CastToGM_Vehicle (Game|GetGameMode)))
  (Variables|/Game/BP/BP_GameControl/BP_GameMode/GM_Vehicle.GM_Vehicle_C|SetIsWin _asgm_vehicle true)
  (bind _returnvalue (UserInterface|CreateWidget "/Game/BP/BP_Menus/WBP_Win.WBP_Win_C" 0 (+ (Variables|/Game/BP/BP_Car/BP_CarEtLink/BP_Ball.BP_Ball_C|GetHowManyCoins _asbp_ball) (Variables|/Game/BP/BP_Car/BP_CarEtLink/BP_Ball1.BP_Ball1_C|GetHowManyCoins _asbp_ball_1))))
  (bind _output_get (Variables|Default|Setwin _returnvalue))
  (bind _output_get_2 (Variables|Default|SetWBP_Timer (Variables|Default|GetWBP_Timer)))
  (Variables|/Game/BP/BP_Menus/WBP_Win.WBP_Win_C|SetfinalTime (Variables|Default|Getwin) (Variables|/Game/BP/BP_Menus/WBP_Timer.WBP_Timer_C|GetCurrentTime _output_get_2))
  (UserInterface|Viewport|AddtoViewport _output_get 0)
  (Game|SetGamePaused true)
  (Input|SetInputModeGameandUI (Game|GetPlayerController 0) (Variables|Default|Getwin) "DoNotLock" true false)
  (Widget|SetKeyboardFocus (Variables|Default|Getwin)))

(event EventBeginPlay
  (bind _returnvalue (Actor|GetActorOfClass "/Game/BP/BP_Car/BP_CarEtLink/BP_Ball.BP_Ball_C"))
  (Variables|Default|SetBall1 _returnvalue)
  (bind _returnvalue_2 (Actor|GetActorOfClass "/Game/BP/BP_Car/BP_CarEtLink/BP_Ball1.BP_Ball1_C"))
  (Variables|Default|SetBP_Ball2 _returnvalue_2)
  (Utilities|FlowControl|Delay 0.1)
  (bind _foundwidgets (Widget|GetAllWidgetsOfClass "/Game/BP/BP_Menus/WBP_Timer.WBP_Timer_C" true))
  (Variables|Default|SetWBP_Timer (Utilities|Array|Get(acopy) _foundwidgets)))

(fn ConstructionScript)