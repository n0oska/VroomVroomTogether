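; Player-controlled physics ball pawn that drives by applying forward force to its sphere while grounded and steers by rotating it in yaw.
; After a short spawn delay it plays force feedback, caches the BP_Link actor, switches the view to the shared BP_CamActor and adds the vehicle input mapping.
; Reset lifts it upright and clears its velocities, while the pause input toggles the pause widget and game pause.
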(event Custom|CustomEvent
  (Transformation|SetActorTransform (Math|Transform|MakeTransform (+ (Transformation|GetActorLocation) "0,0,50.000000") (Math|Rotator|MakeRotator 0.0 0.0 (.yaw (Transformation|GetActorRotation)))))
  ;[0.15 0.15 0.15 0.5] Interrupt any physics-related movement.
  (Class|PrimitiveComponent|SetPhysicsAngularVelocityinDegrees (Variables|Default|GetSphere) "0, 0, 0" false "None")
  (Physics|SetPhysicsLinearVelocity (Variables|Default|GetSphere) "0, 0, 0" false "None"))

(event Custom|CustomEvent_3
  (params (DeltaSeconds :type Float%20%28single-precision%29))
  (Variables|Default|SetOnGround true))

(event Custom|CustomEvent_2
  (Transformation|SetActorTransform (Math|Transform|MakeTransform (+ (Transformation|GetActorLocation) "0,0,50.000000") (Math|Rotator|MakeRotator 0.0 0.0 (.yaw (Transformation|GetActorRotation)))))
  ;[0.15 0.15 0.15 0.5] Interrupt any physics-related movement.
  (Class|PrimitiveComponent|SetPhysicsAngularVelocityinDegrees (Variables|Default|GetSphere) "0, 0, 0" false "None")
  (Physics|SetPhysicsLinearVelocity (Variables|Default|GetSphere) "0, 0, 0" false "None"))

(event Input|EnhancedActionEvents|EnhancedInputActionIA_PauseMenu
  (params (ActionValue :type Boolean) (ElapsedSeconds :type Float%20%28double-precision%29) (TriggeredSeconds :type Float%20%28double-precision%29) (InputAction :type Input%20Action%20Object%20Reference :default "/Game/BP/BP_GameControl/BP_Input/InputAction/IA_PauseMenu.IA_PauseMenu"))
  (bind _returnvalue (Game|GetPlayerController 0))
  (if (not (Variables|Default|GetisPauseMenuOpen))
    (Variables|Default|SetisPauseMenuOpen true)
    (bind _returnvalue_2 (UserInterface|CreateWidget "/Game/BP/BP_Menus/WBP_Pause.WBP_Pause_C" _returnvalue))
    (UserInterface|Viewport|AddtoViewport _returnvalue_2 0)
    (Input|SetInputModeGameandUI _returnvalue (Variables|Default|GetWBP%20Pause) "DoNotLock" false false)
    (Variables|/Script/Engine.PlayerController|SetbShowMouseCursor _returnvalue false)
    (Widget|SetKeyboardFocus (Variables|/Game/BP/BP_Menus/WBP_Pause.WBP_Pause_C|GetVB_Button (Variables|Default|GetWBP%20Pause)))
    (Game|SetGamePaused true)
    (else
      (Variables|Default|SetisPauseMenuOpen false)
      (Widget|RemovefromParent (Variables|Default|GetWBP%20Pause))
      (Game|SetGamePaused false)
      (Input|SetInputModeGameOnly _returnvalue false))))

(event Input|EnhancedActionEvents|EnhancedInputActionIA_Move
  (params (ActionValue :type Vector%202D%20Structure) (ElapsedSeconds :type Float%20%28double-precision%29) (TriggeredSeconds :type Float%20%28double-precision%29) (InputAction :type Input%20Action%20Object%20Reference :default "/Game/BP/BP_GameControl/BP_Input/InputAction/IA_Move.IA_Move"))
  (bind _sphere (Variables|Default|GetSphere))
  (bind _moveforward (Variables|Default|GetMoveForward))
  (bind _returnvalue (Math|Vector|GetForwardVector _sphere))
  (bind _returnvalue_2 (* (.y ActionValue) _moveforward))
  (bind _returnvalue_3 (* _returnvalue_2 _returnvalue))
  (if (Variables|Default|GetOnGround)
    (Development|PrintString (Utilities|String|ToString(Vector) _returnvalue_3))
    (Physics|AddForce (Variables|Default|GetSphere) _returnvalue_3 "None" false)))

(event Input|EnhancedActionEvents|EnhancedInputActionIA_Rotation
  (params (ActionValue :type Float%20%28double-precision%29) (ElapsedSeconds :type Float%20%28double-precision%29) (TriggeredSeconds :type Float%20%28double-precision%29) (InputAction :type Input%20Action%20Object%20Reference :default "/Game/BP/BP_GameControl/BP_Input/InputAction/IA_Rotation.IA_Rotation"))
  (Transformation|AddWorldRotation (Variables|Default|GetSphere) (Math|Rotator|MakeRotator 0.0 0.0 (* ActionValue (Variables|Default|GetRotation))) false false))

(event Input|EnhancedActionEvents|EnhancedInputActionIA_Reset
  (params (ActionValue :type Boolean) (ElapsedSeconds :type Float%20%28double-precision%29) (TriggeredSeconds :type Float%20%28double-precision%29) (InputAction :type Input%20Action%20Object%20Reference :default "/Game/BP/BP_GameControl/BP_Input/InputAction/IA_Reset.IA_Reset"))
  (Transformation|SetActorTransform (Math|Transform|MakeTransform (+ (Transformation|GetActorLocation) "0,0,50.000000") (Math|Rotator|MakeRotator 0.0 0.0 (.yaw (Transformation|GetActorRotation)))))
  ;[0.15 0.15 0.15 0.5] Interrupt any physics-related movement.
  (Class|PrimitiveComponent|SetPhysicsAngularVelocityinDegrees (Variables|Default|GetSphere) "0, 0, 0" false "None")
  (Physics|SetPhysicsLinearVelocity (Variables|Default|GetSphere) "0, 0, 0" false "None"))

(event EventBeginPlay
  (Utilities|FlowControl|Delay 1.5)
  (bind _asplayer_controller (Utilities|Casting|CastToPlayerController (Game|GetInstigatorController)))
  (Game|Feedback|ClientPlayForceFeedback _asplayer_controller "/Game/BP/BP_GameControl/BP_Input/ForceFeedback/FFE_spawn.FFE_spawn" "None" false false false)
  (bind _returnvalue (Actor|GetActorOfClass "/Game/BP/BP_Car/BP_CarEtLink/BP_Link.BP_Link_C"))
  (Variables|Default|SetBP%20Test _returnvalue)
  (bind _returnvalue_2 (Actor|GetActorOfClass "/Game/BP/BP_Camera/BP_CamActor.BP_CamActor_C"))
  (Variables|Default|SetCam _returnvalue_2)
  (Game|Player|SetViewTargetwithBlend (Game|GetPlayerController 0) (Variables|Default|GetCam) 0.0 "VTBlend_Linear" 0.0 false)
  (Input|AddMappingContext (PlayerController|LocalPlayerSubsystems|GetEnhancedInputLocalPlayerSubsystem _asplayer_controller) "/Game/BP/BP_GameControl/BP_Input/IMC/IMC_Vehicle_Default1.IMC_Vehicle_Default1" 0 "(bIgnoreAllPressedKeysUntilRelease=True,bForceImmediately=False,bNotifyUserSettings=False)"))

(fn ConstructionScript)